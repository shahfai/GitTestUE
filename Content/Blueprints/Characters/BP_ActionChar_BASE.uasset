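; Base action character Blueprint that handles taking damage, with a sprite hit flash and removal on defeat.
; AnyDamage passes damage to the BPCVitality component, then destroys the actor if defeated or triggers an orange flash otherwise.
; TriggerFlash sets color and intensity on a dynamic sprite material created at BeginPlay, then a timeline with adjustable play rate lerps the intensity toward zero.
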(event Custom|TriggerFlash
  (params (Flash_Multiplier :type Float%20%28single-precision%29) (Flash_Color :type Linear%20Color%20Structure))
  ;[1 1 1] Triggering flash (Custom Event)
  (Rendering|Material|SetScalarParameterValue (Variables|Default|GetDynamicSpriteMat) "FlashMultiplier" Flash_Multiplier :!class /Script/Engine.MaterialInstanceDynamic)
  (Rendering|Material|SetVectorParameterValue (Variables|Default|GetDynamicSpriteMat) "FlashColor" Flash_Color :!class /Script/Engine.MaterialInstanceDynamic)
  (Components|Timeline|SetPlayRate (Variables|Default|GetFadeSpriteFlash) (Variables|Default|GetSpriteFlashPlayRate))
  (bind _alpha (Timeline|FadeSpriteFlash PlayFromStart)
    (:Update
      (Rendering|Material|SetScalarParameterValue (Variables|Default|GetDynamicSpriteMat) "FlashMultiplier" (Math|Float|Lerp Flash_Multiplier 0.0 _alpha) :!class /Script/Engine.MaterialInstanceDynamic))))

(event EventBeginPlay
  (bind _returnvalue (Rendering|Material|CreateDynamicMaterialInstance (Variables|Default|GetSprite) 0 0 "None" :!class /Script/Engine.PrimitiveComponent))
  (Variables|Default|SetDynamicSpriteMat _returnvalue))

(event Collision|EventActorBeginOverlap
  (params (OtherActor :type Actor%20Object%20Reference)))

(event EventTick
  (params (DeltaSeconds :type Float%20%28single-precision%29)))

(event Game|Damage|EventAnyDamage
  (params (Damage :type Float%20%28single-precision%29) (DamageType :type Damage%20Type%20Object%20Reference) (InstigatedBy :type Controller%20Object%20Reference) (DamageCauser :type Actor%20Object%20Reference))
  (Default|ReceiveDamage (Variables|Default|GetBPC_Vitality) Damage)
  (if (Variables|/Game/Blueprints/Components/BPC_Vitality.BPC_Vitality_C|GetIsDefeated (Variables|Default|GetBPC_Vitality))
    (Actor|DestroyActor)
    (else
      (CallFunction|TriggerFlash 1e+01 "(R=1.000000,G=0.586074,B=0.081205,A=1.000000)"))))

(fn ConstructionScript)